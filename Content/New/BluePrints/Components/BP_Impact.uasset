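; BP_Impact is a component that plays physical-material-specific impact sounds when its owning actor hits something.
; On BeginPlay it enables rigid body collision notifications on the owner's root primitive and binds to OnActorHit.
; Hits above an impulse threshold match the root's first material's physical material against ImpactEvent entries.
; Matches spawn a random attenuated sound at the impact point, with volume scaled by impulse and capped at full.
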(event `self.ReceiveBeginPlay`
  (bind _asprimitive_component (cast `PrimitiveComponent` (`Actor.RootComponent` (`self.GetOwner`)))
    (:`then`
      (`PrimitiveComponent.SetNotifyRigidBodyCollision` _asprimitive_component true)
      (add `Actor.OnActorHit` (`self.GetOwner`) (delegate `HitEvent`)))
    (:`CastFailed`
      (`KismetSystemLibrary.PrintString` "failed"))))

(event `HitEvent`
  (params (SelfActor :type "Actor Object Reference") (OtherActor :type "Actor Object Reference") (NormalImpulse :type "Vector Structure") (Hit :type "HitResult Structure (by ref)"))
  (bind _returnvalue (`KismetMathLibrary.VSize` NormalImpulse))
  (if (> _returnvalue (`self.ImpulseThreshold`))
    (for _array_element (`self.ImpactEvent`)
      (bind (_physicmat _sounds) (break `/Game/New/BluePrints/Components/ImpactStructure` _array_element))
      (if (== _physicmat (`MaterialInterface.GetPhysicalMaterial` (`PrimitiveComponent.GetMaterial` (stale `self.ReceiveBeginPlay` _asprimitive_component) 0)))
        (`GameplayStatics.SpawnSoundAtLocation` (`|GetArrayItem` _sounds (`KismetMathLibrary.RandomIntegerInRange` 0 (- (`KismetArrayLibrary.Array_Length` _sounds) 1))) Hit_ImpactPoint (struct) (`KismetMathLibrary.FMin` (/ _returnvalue (`self.VolumeSensitivity`)) 1.0) 1.0 0.0 "/Game/New/Assets/Sounds/ObjectSoundAttenuation.ObjectSoundAttenuation")))))
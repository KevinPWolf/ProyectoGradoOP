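; BP_ConnectionManager handles account login and sign-up against web endpoints through the VaRest plugin.
; Login and SignUp POST URL-encoded form fields to their URL variables and compare the raw response text to hardcoded success strings.
; Successful login stores the email and clears Logoff on the cached BP_GameInstance, switches to game-only input and opens MainScreen.
; Successful sign-up only prints a message, and failures get no handling beyond printing the response.
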(event `self.ReceiveBeginPlay`
  (bind _asbp_game_instance (cast `/Game/New/BluePrints/BP_GameInstance` (`GameplayStatics.GetGameInstance`)))
  (set `self.GameInst` _asbp_game_instance))

(event `Login`
  (params (MyMail :type String) (MyPassword :type String))
  (bind _returnvalue (`GameplayStatics.GetPlayerController` 0))
  (bind _gameinst (`self.GameInst`))
  (bind _responsecontent (`VaRestRequestJSON.ResponseContent` (`self.Request`)))
  ;[1 1 1] LoginSystem
  (set `self.MyMail` MyMail)
  (set `self.MyPassword` MyPassword)
  (bind _returnvalue_2 (`VaRestRequestJSON.ConstructVaRestRequestExt` "POST" "x_www_form_urlencoded_url"))
  (bind _output_get (set `self.Request` _returnvalue_2))
  (set `self.RequestObject` (`VaRestRequestJSON.GetRequestObject` _output_get))
  (`VaRestJsonObject.SetStringField` (`self.RequestObject`) "username" (`self.MyMail`))
  (`VaRestJsonObject.SetStringField` (`self.RequestObject`) "password" (`self.MyPassword`))
  (`VaRestRequestJSON.ApplyURL` (`self.Request`) (`self.URLLogin`))
  (`KismetSystemLibrary.PrintString` _responsecontent)
  (if (`KismetStringLibrary.EqualEqual_StrStr` _responsecontent "Login-Success")
    (`WidgetBlueprintLibrary.SetInputMode_GameOnly` _returnvalue)
    (set `PlayerController.bShowMouseCursor` false _returnvalue)
    (set `/Game/New/BluePrints/BP_GameInstance.Logoff` false _gameinst)
    (set `/Game/New/BluePrints/BP_GameInstance.UserMail` (`self.MyMail`) _gameinst)
    (`GameplayStatics.OpenLevel` "MainScreen")))

(event `SignUp`
  (params (MyName :type String) (MyMail :type String) (MyPassword :type String) (MyPhone :type String))
  (bind _responsecontent (`VaRestRequestJSON.ResponseContent` (`self.Request`)))
  ;[1 1 1] SignUp System
  (set `self.MyName` MyName)
  (set `self.MyPhone` MyPhone)
  (set `self.MyMail` MyMail)
  (set `self.MyPassword` MyPassword)
  (bind _returnvalue (`VaRestRequestJSON.ConstructVaRestRequestExt` "POST" "x_www_form_urlencoded_url"))
  (bind _output_get (set `self.Request` _returnvalue))
  (set `self.RequestObject` (`VaRestRequestJSON.GetRequestObject` _output_get))
  (`VaRestJsonObject.SetStringField` (`self.RequestObject`) "name" (`self.MyName`))
  (`VaRestJsonObject.SetStringField` (`self.RequestObject`) "phone" (`self.MyPhone`))
  (`VaRestJsonObject.SetStringField` (`self.RequestObject`) "username" (`self.MyMail`))
  (`VaRestJsonObject.SetStringField` (`self.RequestObject`) "password" (`self.MyPassword`))
  (`VaRestRequestJSON.ApplyURL` (`self.Request`) (`self.URLSignUp`))
  (`KismetSystemLibrary.PrintString` _responsecontent true true (struct :`R` 1.0 :`G` 0.038562 :`A` 1.0) 4.0)
  (if (`KismetStringLibrary.EqualEqual_StrStr` _responsecontent "Usuario registrado")
    (`KismetSystemLibrary.PrintString` "El HP lo logro!" true true (struct :`G` 0.40682 :`B` 1.0 :`A` 1.0) 4.0)))

(fn `UserConstructionScript`)
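; Base player for an interior-customization experience with look controls, traced teleporting, gaze-timed interaction, inventory and screenshot capture.
; Camera line traces drive physics-handle grabbing and rotation of movable objects, and open spawned pickers for object meshes and wall or floor materials.
; Picked materials apply to every matching surface in the last overlapped room, with glass on walls preserved.
; The Tutorial level gates surface editing on GameInstance progress.
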(event `/Game/New/BluePrints/ActionInterface.SelectObject`
  (params (Mesh :type "StaticMesh Object Reference"))
  ;[1 1 1] Change Base Object
  (`StaticMeshComponent.SetStaticMesh` (`StaticMeshActor.StaticMeshComponent` (`self.ObjToChange`)) Mesh))

(event `InputAction|ChangeObjButton`
  (params (Key :type "Key Structure"))
  (bind _objpickerref (`self.ObjPickerRef`))
  ;[1 1 1] Change Base Object
  (:`Pressed`
    (`/Engine/EditorBlueprintResources/StandardMacros.FlipFlop`
      (:`A`
        (`self.ChangeBaseObject`))
      (:`B`
        (`/Engine/EditorBlueprintResources/StandardMacros.IsValid` _objpickerref
          (:`Is Valid`
            (`self.K2_DestroyActor` _objpickerref)
            (`self.DisableMouseCursor`)
            (`GameplayStatics.SetGamePaused` false)
            (set `self.OnMenu` false)))))))

(event `/Game/New/BluePrints/ActionInterface.ChangeAction`
  (params (TextureMat :type "MaterialInstance Object Reference") (PartToChange :type Integer))
  ;[1 1 1] Change Materials
  (if (`self.isAWall`)
    (bind _outactors (`GameplayStatics.GetAllActorsOfClass` "/Game/New/BuildingGenerator/AbstractFactory/WallProduct.WallProduct_C"))
    (for _array_element _outactors
      (if (== (`/Game/New/BuildingGenerator/AbstractFactory/AbstractProduct.Room` _array_element) (`self.OverlappedRoom`))
        (bind _staticmeshcomponent (`StaticMeshActor.StaticMeshComponent` _array_element))
        (for (_array_element_2 _array_index) (`MeshComponent.GetMaterials` _staticmeshcomponent)
          (if (not (== _array_element_2 "/Game/New/Assets/Materials/BaseMaterials/Glas.Glas"))
            (`PrimitiveComponent.SetMaterial` _staticmeshcomponent _array_index TextureMat)))))
    (else
      (bind _outactors_2 (`GameplayStatics.GetAllActorsOfClass` "/Game/New/BuildingGenerator/AbstractFactory/FloorCellarProduct.FloorCellarProduct_C"))
      (for _array_element_3 _outactors_2
        (if (== (`/Game/New/BuildingGenerator/AbstractFactory/AbstractProduct.Room` _array_element_3) (`self.OverlappedRoom`))
          (`PrimitiveComponent.SetMaterial` (`StaticMeshActor.StaticMeshComponent` _array_element_3) PartToChange TextureMat))))))

(event `/Game/New/BluePrints/ActionInterface.InspectAction`
  (params (ItemToInspect :type "Actor Object Reference"))
  ;[1 1 1] Inspect Object
  (bind _asbp_moveble (cast `/Game/New/BluePrints/InteractiveObjects/BP_Moveble` ItemToInspect))
  (`self.SetActorHiddenInGame` _asbp_moveble false)
  (`self.K2_SetActorLocation` _asbp_moveble (`SceneComponent.K2_GetComponentLocation` (`self.GrabLocation`)) false false)
  (set `self.isHolding` true)
  (`self.RotateObject`))

(event `/Game/New/BluePrints/ActionInterface.DropAction`
  (params (ItemToDrop :type "Actor Object Reference"))
  (bind _returnvalue (`GameplayStatics.GetObjectClass` ItemToDrop))
  ;[1 1 1] Drop Item
  (`KismetSystemLibrary.PrintString` (`KismetSystemLibrary.GetClassDisplayName` _returnvalue) true true (struct :`R` 1.0 :`G` 0.354083 :`B` 0.36403 :`A` 1.0))
  (`|SpawnActorFromClass` _returnvalue (`SceneComponent.K2_GetComponentToWorld` (`self.DropLocation`)) "AdjustIfPossibleButAlwaysSpawn" "OverrideRootScale" null null))

(event `InputAction|ChangeButton`
  (params (Key :type "Key Structure"))
  (bind _wpickerref (`self.WPickerRef`))
  (bind _fpickerref (`self.FPickerRef`))
  ;[1 1 1] EditWorldObjects
  (:`Pressed`
    (bind _returnvalue (`GameplayStatics.GetCurrentLevelName` true))
    (if (`KismetStringLibrary.EqualEqual_StrStr` _returnvalue "Tutorial")
      (bind _asbp_game_instance (cast `/Game/New/BluePrints/BP_GameInstance` (`GameplayStatics.GetGameInstance`)))
      (if (> (`/Game/New/BluePrints/BP_GameInstance.TutorialP` _asbp_game_instance) 3)
        (`/Engine/EditorBlueprintResources/StandardMacros.FlipFlop` :!label _label
          (:`A`
            (`self.EditWorld`))
          (:`B`
            (`/Engine/EditorBlueprintResources/StandardMacros.IsValid` _wpickerref
              (:`Is Valid`
                (`self.K2_DestroyActor` _wpickerref))
              (:`Is Not Valid`
                (`/Engine/EditorBlueprintResources/StandardMacros.IsValid` _fpickerref
                  (:`Is Valid`
                    (`self.K2_DestroyActor` _fpickerref)))))
            (`self.DisableMouseCursor`)
            (`GameplayStatics.SetGamePaused` false)
            (set `self.OnMenu` false))))
      (else
        (goto _label)))))

(event `self.ReceiveBeginPlay`
  ;[1 1 1] Create HUD
  (set `self.OnMenu` false)
  (set `self.isHolding` false)
  (set `self.isRotating` false)
  (bind _foundwidgets (`WidgetBlueprintLibrary.GetAllWidgetsOfClass` "/Game/New/BluePrints/Widgets/WBP_BasicHUD.WBP_BasicHUD_C" false))
  (set `self.GameHUDRef` (`|GetArrayItem` _foundwidgets)))

(event `InputAction|PickUpButton`
  (params (Key :type "Key Structure"))
  ;[1 1 1] Pickup Items
  (:`Pressed`
    (if (< (`KismetArrayLibrary.Array_Length` (`/Game/New/BluePrints/Widgets/WBP_BasicHUD.Inventory` (`self.GameHUDRef`))) (`self.InventorySize`))
      (set `self.isRotating` false)
      (`self.PickUpItem`))))

(event `self.ReceiveTick`
  (params (DeltaSeconds :type "Float (single-precision)"))
  (bind (_returnvalue_x _returnvalue_y _returnvalue_z) (`KismetMathLibrary.BreakVector` (`SceneComponent.K2_GetComponentLocation` (`self.GrabLocation`))))
  ;[1 1 1] Base Ticks
  (if (`self.isCharging`)
    (`SceneComponent.SetVisibility` (`self.TeleportRef`) true false)
    (`self.PlaceReference`)
    (elif (not (`self.OnMenu`))
      (`PhysicsHandleComponent.SetTargetLocation` (`self.PhysicsHandle`) (`KismetMathLibrary.MakeVector` (+ _returnvalue_x 10.0) _returnvalue_y (- _returnvalue_z 10.0)))
      (`self.TimeBaseGaze`))))

(event `InputAction|InventoryButton`
  (params (Key :type "Key Structure"))
  (bind _gamehudref (`self.GameHUDRef`))
  ;[1 1 1] Toggle Inventory Menu
  (:`Pressed`
    (if (> (`KismetArrayLibrary.Array_Length` (`/Game/New/BluePrints/Widgets/WBP_BasicHUD.Inventory` _gamehudref)) 0)
      (if (`/Game/New/BluePrints/Widgets/WBP_BasicHUD.ActivateInventory` _gamehudref)
        (`/Engine/EditorBlueprintResources/StandardMacros.FlipFlop`
          (:`A`
            (set `/Game/New/BluePrints/Widgets/WBP_BasicHUD.InventoryVisible` "Visible" _gamehudref)
            (bind _asbp_game_instance (cast `/Game/New/BluePrints/BP_GameInstance` (`GameplayStatics.GetGameInstance`)))
            (set `/Game/New/BluePrints/BP_GameInstance.TutMoves` 6 _asbp_game_instance)
            (`self.EnableMouseCursor`))
          (:`B`
            (set `/Game/New/BluePrints/Widgets/WBP_BasicHUD.InventoryVisible` "Hidden" _gamehudref)
            (`self.DisableMouseCursor`)))))))

(event `InputAction|RotateObj`
  (params (Key :type "Key Structure"))
  (bind _gamehudref (`self.GameHUDRef`))
  ;[1 1 1] Rotate Objects
  (:`Pressed`
    (if (`self.isHolding`)
      (`self.RotateObject`)
      (else
        (`/Engine/EditorBlueprintResources/StandardMacros.FlipFlop`
          (:`A`
            (set `/Game/New/BluePrints/Widgets/WBP_BasicHUD.ControllVisibility` "Visible" _gamehudref)
            (bind _returnvalue (`|CreateWidget` "/Game/New/BluePrints/Widgets/WBP_OptionsMenu.WBP_OptionsMenu_C"))
            (`PanelWidget.AddChild` (`/Game/New/BluePrints/Widgets/WBP_BasicHUD.SB_OptionMenu` _gamehudref) _returnvalue)
            (`self.EnableMouseCursor`))
          (:`B`
            (set `/Game/New/BluePrints/Widgets/WBP_BasicHUD.ControllVisibility` "Hidden" _gamehudref)
            (`self.DisableMouseCursor`)))))))

(event `InputAction|InteractionButton` :paused true
  (params (Key :type "Key Structure"))
  ;[1 1 1] Grab and Drop
  (:`Pressed`
    (if (`self.isHolding`)
      (`self.DropObject`)
      (else
        (`self.GrabObject`)))))

(event `InputAxisKey|MouseX`
  (params (AxisValue :type "Float (single-precision)"))
  ;[1 1 1] Editor Camera Movement
  (if (`self.OnMenu`)
    _
    (elif (`self.isRotating`)
      (`self.TurnLeftRight` AxisValue)
      (else
        (`self.AddControllerYawInput` (* (* AxisValue (`GameplayStatics.GetWorldDeltaSeconds`)) (`self.HeadMoveSpeed`)))))))

(event `InputAxis|XAxis`
  (params (AxisValue :type "Float (single-precision)"))
  ;[1 1 1] Rotate Joystick
  (if (`self.isRotating`)
    (`self.TurnLeftRight` AxisValue)))

(event `InputAxisKey|MouseY`
  (params (AxisValue :type "Float (single-precision)"))
  ;[1 1 1] Editor Camera Movement
  (if (`self.OnMenu`)
    _
    (elif (`self.isRotating`)
      (`self.TurnUp` AxisValue)
      (else
        (`self.AddControllerPitchInput` (* (* AxisValue (`GameplayStatics.GetWorldDeltaSeconds`)) (* (`self.HeadMoveSpeed`) -1.0)))))))

(event `InputAction|TeleportButton`
  (params (Key :type "Key Structure"))
  ;[1 1 1] Teleport Movement
  (:`Pressed`
    (set `self.isCharging` true))
  (:`Released`
    (set `self.isCharging` false)
    (`self.Teleport`)))

(event `InputAxis|YAxis`
  (params (AxisValue :type "Float (single-precision)"))
  ;[1 1 1] Rotate Joystick
  (if (`self.isRotating`)
    (`self.TurnUp` AxisValue)))

(event `self.Capsule.OnComponentBeginOverlap`
  (params (OverlappedComponent :type "PrimitiveComponent Object Reference") (OtherActor :type "Actor Object Reference") (OtherComp :type "PrimitiveComponent Object Reference") (OtherBodyIndex :type Integer) (bFromSweep :type Boolean) (SweepResult :type "HitResult Structure (by ref)"))
  (bind _asabstract_product (cast `/Game/New/BuildingGenerator/AbstractFactory/AbstractProduct` OtherActor))
  (bind _output_get (set `self.OverlappedRoom` (`/Game/New/BuildingGenerator/AbstractFactory/AbstractProduct.Room` _asabstract_product)))
  (`KismetSystemLibrary.PrintString` (`KismetStringLibrary.Concat_StrStr` "ActualRoom:  " (`KismetStringLibrary.Conv_IntToString` _output_get))))

(event `Key|X`
  (params (Key :type "Key Structure"))
  (bind _returnvalue (`VictoryBPFunctionLibrary.VictoryPaths__ScreenShotsDir`))
  (bind _returnvalue_2 (`GameplayStatics.GetPlayerController` 0))
  (:`Pressed`
    (bind _foundwidgets (`WidgetBlueprintLibrary.GetAllWidgetsOfClass` "/Game/New/BluePrints/Widgets/WBP_Cellphone_Screenshoots.WBP_Cellphone_Screenshoots_C"))
    (`Widget.RemoveFromParent` _foundwidgets)
    (`SceneComponent.K2_SetWorldTransform` (`self.GrabLocation`) (`KismetMathLibrary.MakeTransform` (0.0 0.0 0.0) (struct) (0.1 0.1 0.1)) false false)
    (`ScaleImage.TakeScreenshot` 200 200)
    (bind _asbp_game_instance (cast `/Game/New/BluePrints/BP_GameInstance` (`GameplayStatics.GetGameInstance`)))
    (bind _returnvalue_3 (`KismetStringLibrary.Concat_StrStr` (`/Game/New/BluePrints/BP_GameInstance.UserMail` _asbp_game_instance) "_scrnsht_" (`KismetStringLibrary.Conv_IntToString` (`self.ScreenShootNumber`))))
    (`VictoryBPFunctionLibrary.ScreenShots_Rename_Move_Most_Recent` _returnvalue_3 _returnvalue)
    (`KismetSystemLibrary.PrintString` _returnvalue_3)
    (bind _returnvalue_4 (`|CreateWidget` "/Game/New/BluePrints/Widgets/WBP_Cellphone_Screenshoots.WBP_Cellphone_Screenshoots_C"))
    (`/Game/New/BluePrints/Widgets/WBP_Cellphone_Screenshoots.OpenScreenshoot` _returnvalue_4 _returnvalue _returnvalue_3)
    (`UserWidget.AddToViewport` _returnvalue_4 0)
    (`/Engine/EditorBlueprintResources/StandardMacros.IncrementInt` (`self.ScreenShootNumber`)
      (:`  `
        (`WidgetBlueprintLibrary.SetInputMode_GameAndUIEx` _returnvalue_2 _returnvalue_4 "DoNotLock" false)
        (set `PlayerController.bShowMouseCursor` true _returnvalue_2)))))

(fn `ChangeBaseObject`
  (bind _outhit (`self.LineTraceForward` (`self.Camera`) (`|MakeArray` "ObjectTypeQuery9" :!type "EObjectTypeQuery Enum")))
  (bind (_bblockinghit _binitialoverlap _time _distance _location _impactpoint _normal _impactnormal _physmat _hitactor) (`GameplayStatics.BreakHitResult` _outhit))
  (bind _asobject_product (cast `/Game/New/BuildingGenerator/AbstractFactory/ObjectProduct` _hitactor))
  (set `self.ObjToChange` _asobject_product)
  (set `self.OnMenu` true)
  (bind _returnvalue (`|SpawnActorFromClass` "/Game/New/BluePrints/Widgets/BP_ObjectPicker.BP_ObjectPicker_C" (`KismetMathLibrary.MakeTransform` (+ _impactpoint (`self.ForwarePosition`))) "Undefined" "OverrideRootScale" null null))
  (bind _output_get (set `self.ObjPickerRef` _returnvalue))
  (bind _foundwidgets (`WidgetBlueprintLibrary.GetAllWidgetsOfClass` (`/Game/New/BluePrints/Widgets/BP_ObjectPicker.PickerMenu` _output_get) "/Game/New/BluePrints/Widgets/WBP_ObjectPicker.WBP_ObjectPicker_C" false))
  (`/Game/New/BluePrints/Widgets/WBP_ObjectPicker.RefreshInventory` _foundwidgets))

(fn `DisableMouseCursor`
  (bind _returnvalue (`GameplayStatics.GetPlayerController` 0))
  (`WidgetBlueprintLibrary.SetInputMode_GameOnly` _returnvalue)
  (set `PlayerController.bShowMouseCursor` false _returnvalue))

(fn `DropObject`
  (bind _physobject (`self.PhysObject`))
  (`PhysicsHandleComponent.ReleaseComponent` (`self.PhysicsHandle`))
  (set `self.isHolding` false)
  (`PrimitiveComponent.SetAllPhysicsLinearVelocity` _physobject (0.0 0.0 0.0) false)
  (`PrimitiveComponent.SetAngularDamping` _physobject 0.0)
  (`PrimitiveComponent.SetEnableGravity` _physobject true)
  (set `self.isRotating` false)
  (set `/Game/New/BluePrints/InteractiveObjects/BP_Moveble.IsGrabed?` false (`self.MovebleObj`)))

(fn `EditWorld`
  (bind _outhit (`self.LineTraceForward` (`self.Camera`) (`|MakeArray` "ObjectTypeQuery8" :!type "EObjectTypeQuery Enum")))
  (bind (_bblockinghit _binitialoverlap _time _distance _location _impactpoint _normal _impactnormal _physmat _hitactor) (`GameplayStatics.BreakHitResult` _outhit))
  (cast `/Game/New/BuildingGenerator/AbstractFactory/WallProduct` _hitactor
    (:`then`
      (set `self.OnMenu` true)
      (bind _returnvalue (+ _impactpoint (`self.ForwarePosition`)))
      (bind _returnvalue_2 (`|SpawnActorFromClass` "/Game/New/BluePrints/Widgets/BP_WallTexturePicker.BP_WallTexturePicker_C" (`KismetMathLibrary.MakeTransform` _returnvalue) "Undefined" "OverrideRootScale" null null))
      (bind _output_get (set `self.WPickerRef` _returnvalue_2))
      (bind _foundwidgets (`WidgetBlueprintLibrary.GetAllWidgetsOfClass` (`/Game/New/BluePrints/Widgets/BP_WallTexturePicker.PickerMenu` _output_get) "/Game/New/BluePrints/Widgets/WBP_WallTexturePicker.WBP_WallTexturePicker_C" false))
      (`/Game/New/BluePrints/Widgets/WBP_WallTexturePicker.RefreshInventory` _foundwidgets)
      (set `self.isAWall` true))
    (:`CastFailed`
      (cast `/Game/New/BuildingGenerator/AbstractFactory/FloorCellarProduct` _hitactor)
      (set `self.OnMenu` true)
      (bind _returnvalue_3 (`|SpawnActorFromClass` "/Game/New/BluePrints/Widgets/BP_FloorTexturePicker.BP_FloorTexturePicker_C" (`KismetMathLibrary.MakeTransform` _returnvalue) "Undefined" "OverrideRootScale" null null))
      (bind _output_get_2 (set `self.FPickerRef` _returnvalue_3))
      (bind _foundwidgets_2 (`WidgetBlueprintLibrary.GetAllWidgetsOfClass` (`/Game/New/BluePrints/Widgets/BP_FloorTexturePicker.PickerMenu` _output_get_2) "/Game/New/BluePrints/Widgets/WBP_FloorTexturePicker.WBP_FloorTexturePicker_C" false))
      (`/Game/New/BluePrints/Widgets/WBP_FloorTexturePicker.RefreshInventory` _foundwidgets_2)
      (set `self.isAWall` false))))

(fn `EnableMouseCursor`
  (`WidgetBlueprintLibrary.SetInputMode_GameAndUIEx` (`GameplayStatics.GetPlayerController` 0) (`/Game/New/BluePrints/Widgets/WBP_BasicHUD.Slot_0` (`self.GameHUDRef`))))

(fn `GrabObject`
  (bind _physobject (`self.PhysObject`))
  (bind _outhit (`self.LineTraceForward` (`self.Camera`) (`|MakeArray` "ObjectTypeQuery7" :!type "EObjectTypeQuery Enum")))
  (bind (_bblockinghit _binitialoverlap _time _distance _location _impactpoint _normal _impactnormal _physmat _hitactor _hitcomponent) (`GameplayStatics.BreakHitResult` _outhit))
  (if (`SceneComponent.IsSimulatingPhysics` _hitcomponent "None")
    (bind _asbp_moveble (cast `/Game/New/BluePrints/InteractiveObjects/BP_Moveble` _hitactor))
    (set `self.MovebleObj` _asbp_moveble)
    (bind _output_get (set `self.PhysObject` _hitcomponent))
    (`PhysicsHandleComponent.GrabComponentAtLocation` (`self.PhysicsHandle`) _output_get "None" (`SceneComponent.K2_GetComponentLocation` _hitcomponent))
    (set `self.isHolding` true)
    (`PrimitiveComponent.SetAngularDamping` _physobject 10.0)
    (`PrimitiveComponent.SetEnableGravity` _physobject false)
    (set `/Game/New/BluePrints/InteractiveObjects/BP_Moveble.IsGrabed?` true (`self.MovebleObj`))))

(fn `Interact`
  (bind _interactiveobject (`self.InteractiveObject`))
  (bind _timerref (`self.TimerRef`))
  (`/Engine/EditorBlueprintResources/StandardMacros.IsValid` _interactiveobject
    (:`Is Valid`
      (`/Game/New/BluePrints/InteractiveObjects/BP_InteractiveBase.Activate` _interactiveobject)
      (`/Engine/EditorBlueprintResources/StandardMacros.IsValid` _timerref
        (:`Is Valid`
          (`self.K2_DestroyActor` _timerref))))))

(fn `LineTraceForward`
  (params (InitialPnt :type "SceneComponent Object Reference") (ObjectTypes :type "Array of EObjectTypeQuery Enum (by ref)"))
  (returns (OutHit :type "HitResult Structure"))
  (bind _returnvalue (`SceneComponent.K2_GetComponentLocation` InitialPnt))
  (bind _outhit (`KismetSystemLibrary.LineTraceSingleForObjects` _returnvalue (+ _returnvalue (* (`KismetMathLibrary.GetForwardVector` (`SceneComponent.K2_GetComponentRotation` InitialPnt)) 10000.0)) ObjectTypes))
  (return _outhit))

(fn `PlaceReference`
  (bind (_returnvalue_roll _returnvalue_pitch _returnvalue_yaw) (`KismetMathLibrary.BreakRotator` (`SceneComponent.K2_GetComponentRotation` (`self.Camera`))))
  (bind _outhit (`self.LineTraceForward` (`self.Camera`) (`|MakeArray` "ObjectTypeQuery8" "ObjectTypeQuery9" :!type "EObjectTypeQuery Enum")))
  (bind (_bblockinghit _binitialoverlap _time _distance _location _impactpoint _normal) (`GameplayStatics.BreakHitResult` _outhit))
  (if (> (`KismetMathLibrary.Dot_VectorVector` _normal (0.0 0.0 1.0)) 0.1)
    (bind _output_get (set `self.TeleportLocation` _location))
    (`SceneComponent.K2_SetWorldTransform` (`self.TeleportRef`) (`KismetMathLibrary.MakeTransform` (`KismetMathLibrary.MakeVector` (.x _output_get) (.y _output_get) (+ (.z _output_get) 5.0)) (`KismetMathLibrary.MakeRotator` _returnvalue_roll 0.0 (+ _returnvalue_yaw -90.0)) (0.2 0.2 0.2)) false false)))

(fn `RotateObject`
  (if (`self.isHolding`)
    (if (`self.isRotating`)
      (set `self.isRotating` false)
      (else
        (set `self.isRotating` true)))
    (else
      (set `self.isRotating` false))))

(fn `Teleport`
  (bind (_teleportlocation_x _teleportlocation_y _teleportlocation_z) (`KismetMathLibrary.BreakVector` (`self.TeleportLocation`)))
  (`self.K2_SetActorLocation` (`KismetMathLibrary.MakeVector` _teleportlocation_x _teleportlocation_y (+ _teleportlocation_z (`CapsuleComponent.CapsuleHalfHeight` (`self.Capsule`)))))
  (`SceneComponent.SetVisibility` (`self.TeleportRef`) false false))

(fn `TimeBaseGaze`
  (bind _timerref (`self.TimerRef`))
  (bind _outhit (`self.LineTraceForward` (`self.Camera`) (`|MakeArray` "ObjectTypeQuery8" :!type "EObjectTypeQuery Enum")))
  (bind (_bblockinghit _binitialoverlap _time _distance _location _impactpoint _normal _impactnormal _physmat _hitactor) (`GameplayStatics.BreakHitResult` _outhit))
  (if _bblockinghit
    (bind _asbp_interactive_base (cast `/Game/New/BluePrints/InteractiveObjects/BP_InteractiveBase` _hitactor)
      (:`then`
        (set `self.InteractiveObject` _asbp_interactive_base)
        (if (not (== (`self.InteractiveObject`) (`self.FocusedObject`)))
          (set `self.FocusedObject` (`self.InteractiveObject`))
          (`KismetSystemLibrary.K2_ClearAndInvalidateTimerHandle` (`self.FocusTimer`))
          (bind _returnvalue (`KismetSystemLibrary.K2_SetTimer` null "Interact" (`self.TimerLength`)))
          (set `self.FocusTimer` _returnvalue)
          (`/Engine/EditorBlueprintResources/StandardMacros.IsValid` (`self.TimerRef`)
            (:`Is Not Valid`
              (bind _returnvalue_2 (`|SpawnActorFromClass` "/Game/New/BluePrints/BP_RadialTimer.BP_RadialTimer_C" (`KismetMathLibrary.MakeTransform` (+ (`self.K2_GetActorLocation` (`self.FocusedObject`)) (`self.ForwarePosition`))) "Undefined" "OverrideRootScale" null null))
              (set `self.TimerRef` _returnvalue_2)))))
      (:`CastFailed`
        (set `self.InteractiveObject` null :!label _label)
        (set `self.FocusedObject` null)
        (`KismetSystemLibrary.K2_ClearAndInvalidateTimerHandle` (`self.FocusTimer`))
        (`/Engine/EditorBlueprintResources/StandardMacros.IsValid` _timerref
          (:`Is Valid`
            (`self.K2_DestroyActor` _timerref)))))
    (else
      (goto _label))))

(fn `TurnLeftRight`
  (params (`Z (Yaw)` :type "Float (double-precision)"))
  (bind _physobject (`self.PhysObject`))
  (`SceneComponent.K2_SetWorldRotation` _physobject (`KismetMathLibrary.ComposeRotators` (`SceneComponent.K2_GetComponentRotation` _physobject) (`KismetMathLibrary.MakeRotator` 0.0 0.0 (* `Z (Yaw)` -1.0))) false false))

(fn `TurnUp`
  (params (`X (Roll)` :type "Float (double-precision)"))
  (bind _physobject (`self.PhysObject`))
  (`SceneComponent.K2_SetWorldRotation` _physobject (`KismetMathLibrary.ComposeRotators` (`SceneComponent.K2_GetComponentRotation` _physobject) (`KismetMathLibrary.MakeRotator` `X (Roll)` `X (Roll)`)) false false))

(fn `UserConstructionScript`)
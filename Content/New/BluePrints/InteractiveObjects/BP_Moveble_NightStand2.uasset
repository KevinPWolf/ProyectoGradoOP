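; Movable nightstand actor whose visibility and height follow the tutorial phase stored in the game instance.
; BeginPlay caches BP_GameInstance, and Tick polls its TutorialP value.
; Phase 1 hides the mesh and teleports the actor to a raised height, while phase 2 shows it and teleports it down to near zero height.
; Each teleport keeps X and Y and runs only once through its own DoOnce.
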(event `self.ReceiveBeginPlay`
  (`parent.ReceiveBeginPlay`)
  (bind _asbp_game_instance (cast `/Game/New/BluePrints/BP_GameInstance` (`GameplayStatics.GetGameInstance`)))
  (set `self.GameInst` _asbp_game_instance))

(event `self.ReceiveTick`
  (params (DeltaSeconds :type "Float (single-precision)"))
  (bind (_returnvalue_x _returnvalue_y) (`KismetMathLibrary.BreakVector` (`self.K2_GetActorLocation`)))
  (bind _staticmesh (`self.StaticMesh`))
  (bind _tutorialp (`/Game/New/BluePrints/BP_GameInstance.TutorialP` (`self.GameInst`)))
  (if (== _tutorialp 1)
    (`SceneComponent.SetVisibility` _staticmesh false false)
    (`/Engine/EditorBlueprintResources/StandardMacros.DoOnce` false
      (:`Completed`
        (`self.K2_SetActorLocation` (`KismetMathLibrary.MakeVector` _returnvalue_x _returnvalue_y 350.0) false true)))
    (elif (== _tutorialp 2)
      (`SceneComponent.SetVisibility` _staticmesh true false)
      (`/Engine/EditorBlueprintResources/StandardMacros.DoOnce` false
        (:`Completed`
          (`self.K2_SetActorLocation` (`KismetMathLibrary.MakeVector` _returnvalue_x _returnvalue_y 3.0) false true))))))

(fn `UserConstructionScript`
  (`parent.UserConstructionScript`))
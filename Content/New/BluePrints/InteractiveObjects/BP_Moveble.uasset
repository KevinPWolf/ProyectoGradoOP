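; BP_Moveble is a grabbable interactive object that the player can pick up into the inventory.
; On BeginPlay it records itself in its ItemInfo struct, caches the player as BP_PlayerBase and binds to that player's PickUpItem dispatcher.
; When the dispatcher fires and the object is grabbed with collision enabled, it adds ItemInfo to the HUD's inventory, refreshes it and destroys itself.
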(event `self.ReceiveBeginPlay`
  ;[1 1 1] PickUp Initial
  (setmembers `/Game/New/BluePrints/InventoryStruct` :`StructRef` (`self.ItemInfo`) :`Item` self)
  (bind _asbp_player_base (cast `/Game/New/BluePrints/BP_PlayerBase` (`GameplayStatics.GetPlayerPawn` 0)))
  (bind _output_get (set `self.PlayerRef` _asbp_player_base))
  (add `/Game/New/BluePrints/BP_PlayerBase.PickUpItem` _output_get (delegate `PickUpItem_Event_0`)))

(event `PickUpItem_Event_0`
  (bind _gamehudref (`/Game/New/BluePrints/BP_PlayerBase.GameHUDRef` (`self.PlayerRef`)))
  ;[1 1 1] Pickup And Add Items
  (if (and (`self.GetActorEnableCollision`) (`self.IsGrabed?`))
    (`KismetArrayLibrary.Array_Add` (`/Game/New/BluePrints/Widgets/WBP_BasicHUD.Inventory` _gamehudref) (`self.ItemInfo`))
    (`/Game/New/BluePrints/Widgets/WBP_BasicHUD.RefreshInventory` _gamehudref)
    (`self.K2_DestroyActor`)))

(fn `UserConstructionScript`)
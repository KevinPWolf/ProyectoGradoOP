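; BP_InteractiveMovMachine is an interactive object that opens a movement selection menu when activated.
; On BeginPlay it caches the player pawn and game instance.
; Activation only works once a song is selected in the game instance: it spawns a BP_MovementSelector actor at an offset, flags the player as in a menu, and switches input to Game and UI focused on the selector widget.
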(event `self.ReceiveBeginPlay`
  (`parent.ReceiveBeginPlay`)
  (bind _asbp_player_base (cast `/Game/New/BluePrints/BP_PlayerBase` (`GameplayStatics.GetPlayerPawn` 0)))
  (set `self.Player` _asbp_player_base)
  (bind _asbp_game_instance (cast `/Game/New/BluePrints/BP_GameInstance` (`GameplayStatics.GetGameInstance`)))
  (set `self.GameInst` _asbp_game_instance))

(event `self.Activate`
  (bind _returnvalue_location (`KismetMathLibrary.BreakTransform` (`self.GetTransform`)))
  (if (`/Game/New/BluePrints/BP_GameInstance.SongSelected?` (`self.GameInst`))
    (bind _returnvalue (`|SpawnActorFromClass` "/Game/New/BluePrints/Widgets/BP_MovementSelector.BP_MovementSelector_C" (`KismetMathLibrary.MakeTransform` (+ _returnvalue_location (`self.Offset`))) "Undefined" "OverrideRootScale" null null))
    (set `self.WidgetMov` _returnvalue)
    (set `/Game/New/BluePrints/BP_PlayerBase.OnMenu` true (`self.Player`))
    (bind _foundwidgets (`WidgetBlueprintLibrary.GetAllWidgetsOfClass` "/Game/New/BluePrints/Widgets/WBP_MovementSelector.WBP_MovementSelector_C" false))
    (`WidgetBlueprintLibrary.SetInputMode_GameAndUIEx` (`GameplayStatics.GetPlayerController` 0) (`|GetArrayItem` _foundwidgets))))

(fn `UserConstructionScript`
  (`parent.UserConstructionScript`))
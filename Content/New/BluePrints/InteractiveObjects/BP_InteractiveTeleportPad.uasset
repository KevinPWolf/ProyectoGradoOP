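; BP_InteractiveTeleportPad is an interactive object that teleports the player to itself when activated.
; BeginPlay calls the parent logic, then casts the first player pawn to BP_PlayerBase and caches it.
; Activate moves that player to just above the pad's own location, keeping the player's current rotation.
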(event `self.ReceiveBeginPlay`
  (`parent.ReceiveBeginPlay`)
  (bind _asbp_player_base (cast `/Game/New/BluePrints/BP_PlayerBase` (`GameplayStatics.GetPlayerPawn` 0)))
  (set `self.Player` _asbp_player_base))

(event `self.Activate`
  (bind _player (`self.Player`))
  (`self.K2_TeleportTo` _player (+ (`self.K2_GetActorLocation`) (0.0 0.0 120.0)) (`self.K2_GetActorRotation` _player)))

(fn `UserConstructionScript`
  (`parent.UserConstructionScript`))
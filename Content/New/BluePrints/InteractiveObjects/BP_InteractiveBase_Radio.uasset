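; Interactive radio object that opens a music selection menu when activated.
; BeginPlay caches the player pawn as a BP_PlayerBase.
; Activate spawns a BP_MusicSelector at an offset from the radio, clears WidgetMov and flags the player as in a menu.
; It then switches input to Game and UI, focusing the first WBP_RadioPlayer widget found by a class search rather than a stored reference.
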(event `self.ReceiveBeginPlay`
  (bind _asbp_player_base (cast `/Game/New/BluePrints/BP_PlayerBase` (`GameplayStatics.GetPlayerPawn` 0)))
  (set `self.Player` _asbp_player_base))

(event `self.Activate`
  (bind _returnvalue_location (`KismetMathLibrary.BreakTransform` (`self.GetTransform`)))
  (`|SpawnActorFromClass` "/Game/New/BluePrints/Widgets/BP_MusicSelector.BP_MusicSelector_C" (`KismetMathLibrary.MakeTransform` (+ _returnvalue_location (`self.Offset`))) "Undefined" "OverrideRootScale" null null)
  (set `self.WidgetMov` null)
  (set `/Game/New/BluePrints/BP_PlayerBase.OnMenu` true (`self.Player`))
  (bind _foundwidgets (`WidgetBlueprintLibrary.GetAllWidgetsOfClass` "/Game/New/BluePrints/Widgets/WBP_RadioPlayer.WBP_RadioPlayer_C" false))
  (`WidgetBlueprintLibrary.SetInputMode_GameAndUIEx` (`GameplayStatics.GetPlayerController` 0) (`|GetArrayItem` _foundwidgets)))

(fn `UserConstructionScript`
  (`parent.UserConstructionScript`))